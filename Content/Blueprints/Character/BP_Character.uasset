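; Player character Blueprint that creates the HUD, handles walk input and swaps between three AR4 weapon variants on number keys.
; Walk input sets a flag and refreshes movement state, while weapon swaps destroy the current weapon and initialize another by name.
; Tick plays a world camera shake at the first-person camera while the current weapon fires.
; Camera boom setup and timer-driven height slide logic are left disconnected and never run.
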(event `self.ReceiveTick`
  (params (DeltaSeconds :type "Float (single-precision)"))
  (bind _returnvalue (`self.GetCurrentWeapon`))
  (`/Engine/EditorBlueprintResources/StandardMacros.IsValid` _returnvalue
    (:`Is Valid`
      (if (`WeaponDefault.WeaponFiring` _returnvalue)
        (`self.CameraShakeEvent`)))))

(event `self.ReceiveBeginPlay`
  (bind _returnvalue (`|CreateWidget` "/Game/Blueprints/Character/BP_HUD.BP_HUD_C"))
  (`UserWidget.AddToViewport` _returnvalue 0))

(event `InputAction|Walk`
  (params (Key :type "Key Structure"))
  ;[1 1 1] State Changer
  (:`Pressed`
    (set `self.WalkEnable` true)
    (`self.ChangeMovementState` :!label _label))
  (:`Released`
    (set `self.WalkEnable` false)
    (goto _label)))

(event `Key|One`
  (params (Key :type "Key Structure"))
  (:`Pressed`
    (bind _returnvalue (`self.GetCurrentWeapon`))
    (`self.K2_DestroyActor` _returnvalue)
    (`self.InitWeapon` "AR4")))

(event `Key|Two`
  (params (Key :type "Key Structure"))
  (:`Pressed`
    (bind _returnvalue (`self.GetCurrentWeapon`))
    (`self.K2_DestroyActor` _returnvalue)
    (`self.InitWeapon` "AR4E")))

(event `Key|Three`
  (params (Key :type "Key Structure"))
  (:`Pressed`
    (bind _returnvalue (`self.GetCurrentWeapon`))
    (`self.K2_DestroyActor` _returnvalue)
    (`self.InitWeapon` "AR4C")))

(fn `Camera Slide`
  (params (Value :type "Float (double-precision)")))

(fn `CameraShakeEvent`
  (`GameplayStatics.PlayWorldCameraShake` "/Game/Blueprints/Game/BP_CameraShake.BP_CameraShake_C" (`SceneComponent.K2_GetComponentLocation` (`self.FirstPersonCamera`)) 0.0 2.0))

(fn `CameraSlideSmoothTick`)

(fn `UserConstructionScript`)